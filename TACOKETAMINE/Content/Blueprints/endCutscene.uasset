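; End-cutscene trigger that fires when the first-person character overlaps its R component.
; The overlap disables the character's movement, then gathers every PoweredLights actor and makes its point light visible.
; The EndPlayInEditor sound plays inside that loop, once per light.
; Nodes for destroying the actor, switching to UI-only input and zeroing velocity are unconnected and never run.
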(event OnComponentBeginOverlap(r)
  (params (OverlappedComponent :type Primitive%20Component%20Object%20Reference) (OtherActor :type Actor%20Object%20Reference) (OtherComp :type Primitive%20Component%20Object%20Reference) (OtherBodyIndex :type Integer) (bFromSweep :type Boolean) (SweepResult :type Hit%20Result%20Structure%20%28by%20ref%29))
  (bind _asbp_first_person_character (Utilities|Casting|CastToBP_FirstPersonCharacter OtherActor))
  (Pawn|Components|CharacterMovement|DisableMovement (Variables|/Script/Engine.Character|GetCharacterMovement _asbp_first_person_character))
  (bind _outactors (Actor|GetAllActorsOfClass "/Game/prop/generator/poweredLights.poweredLights_C"))
  (for _array_element _outactors
    (Rendering|SetVisibility (Variables|/Script/Engine.PointLight|GetPointLightComponent _array_element) true false)
    (Audio|PlaySound2D "/Engine/EditorSounds/GamePreview/EndPlayInEditor.EndPlayInEditor" 1.0 1.0 0.0 0 0)))

(event EventBeginPlay)

(event Collision|EventActorBeginOverlap
  (params (OtherActor :type Actor%20Object%20Reference)))

(event EventTick
  (params (DeltaSeconds :type Float%20%28single-precision%29)))

(fn ConstructionScript)