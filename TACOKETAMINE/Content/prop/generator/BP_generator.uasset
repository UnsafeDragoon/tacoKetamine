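; BP_generator is an interactable generator prop that switches the level's powered lights on and off.
; Each Interact alternates via FlipFlop between off and on, starting with off, turning its own indicator light red or green.
; It writes GeneratorPowerOn directly on the player's BP_FirstPersonCharacter and toggles PointLightComponent visibility on every PoweredLights actor found with GetAllActorsOfClass.
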(event EventBeginPlay)

(event Collision|EventActorBeginOverlap
  (params (OtherActor :type Actor%20Object%20Reference)))

(event EventTick
  (params (DeltaSeconds :type Float%20%28single-precision%29)))

(event EventInteract
  (bind _pointlight (Variables|Default|GetPointLight))
  (bind _asbp_first_person_character (Utilities|Casting|CastToBP_FirstPersonCharacter (Game|GetPlayerCharacter 0)))
  (Utilities|FlowControl|FlipFlop
    (:A
      (Rendering|Components|Light|SetLightColor _pointlight "(R=1.000000,G=0.000000,B=0.000000,A=1.000000)" true)
      (Variables|/Game/FirstPerson/Blueprints/BP_FirstPersonCharacter.BP_FirstPersonCharacter_C|SetgeneratorPowerOn? _asbp_first_person_character false)
      (bind _outactors (Actor|GetAllActorsOfClass "/Game/prop/generator/poweredLights.poweredLights_C"))
      (for _array_element _outactors
        (Rendering|SetVisibility (Variables|/Script/Engine.PointLight|GetPointLightComponent _array_element) false false)))
    (:B
      (Rendering|Components|Light|SetLightColor _pointlight "(R=0.123674,G=1.000000,B=0.000000,A=1.000000)" true)
      (Variables|/Game/FirstPerson/Blueprints/BP_FirstPersonCharacter.BP_FirstPersonCharacter_C|SetgeneratorPowerOn? _asbp_first_person_character true)
      (bind _outactors_2 (Actor|GetAllActorsOfClass "/Game/prop/generator/poweredLights.poweredLights_C"))
      (for _array_element_2 _outactors_2
        (Rendering|SetVisibility (Variables|/Script/Engine.PointLight|GetPointLightComponent _array_element_2) true false)))))

(fn ConstructionScript)